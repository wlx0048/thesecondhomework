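; A GameState Blueprint that keeps a match countdown timer and resets player scores.
; The timedesc event, guarded by a running flag, uses a looping one-second Delay to decrement the remaining time until it reaches zero.
; The 初始化 (initialize) function resets the timer to sixty seconds and zeroes PlayerScore on each MyPlayerState in PlayerArray.
; Its RepNotify handlers and the 倒计时 (countdown) function are empty.
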(event Custom|timedesc
  (if (not (Variables|Default|Get是否开始倒计时))
    (Variables|Default|Set是否开始倒计时 true)
    (Utilities|FlowControl|Delay 1.0 :!label _label)
    (bind _output_get (Variables|Default|Set剩余时间 (- (Variables|Default|Get剩余时间) 1)))
    (if (== _output_get 0)
      (Variables|Default|Set是否开始倒计时 false)
      (else
        (goto _label)))))

(fn ConstructionScript)

(fn OnRepGameStartTimer)

(fn OnRepRandomTimerValue1)

(fn 倒计时)

(fn OnRep剩余时间)

(fn 初始化
  (Variables|Default|Set剩余时间 60)
  (for _array_element (Variables|/Script/Engine.GameStateBase|GetPlayerArray (Game|GetGameState))
    (bind _asmy_player_state (Utilities|Casting|CastToMyPlayerState _array_element))
    (Variables|/Game/Blueprints/MyPlayerState.MyPlayerState_C|SetPlayerScore _asmy_player_state 0)))