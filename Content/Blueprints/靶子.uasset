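; Shooting target actor (靶子) that moves along a timeline path and awards score to the player who damages it.
; On BeginPlay, 移动 runs a timeline that lerps X and Z offsets from its starting location, and a dynamic material is created for the Sphere.
; AnyDamage increments the instigator's MyPlayerState score and briefly flashes the sphere red before resetting it to white, printing a debug string if the cast fails.
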(event Custom|移动
  (Variables|Default|Set位置 (Transformation|GetActorLocation self))
  (bind _新建轨道_0 (Timeline|时间轴_0 Play)
    (:Update
      (Transformation|SetActorLocation (Math|Vector|MakeVector (+ (Math|Float|Lerp -4e+02 4e+02 _新建轨道_0) (.x (Variables|Default|Get位置))) (.y (Variables|Default|Get位置)) (+ (Math|Float|Lerp 0.0 3e+02 _新建轨道_0) (.z (Variables|Default|Get位置)))) false false))))

(event EventBeginPlay
  (bind _sphere (Variables|Default|GetSphere))
  (CallFunction|移动)
  (bind _returnvalue (Rendering|Material|CreateDynamicMaterialInstance (Rendering|Material|GetMaterial _sphere 0) "None" "None" :!class /Script/Engine.KismetMaterialLibrary))
  (Variables|Default|Setdynamic%20material _returnvalue)
  (Rendering|Material|SetMaterial _sphere 0 _returnvalue))

(event Collision|EventActorBeginOverlap
  (params (OtherActor :type Actor%20Object%20Reference)))

(event EventTick
  (params (DeltaSeconds :type Float%20%28single-precision%29)))

(event Game|Damage|EventAnyDamage
  (params (Damage :type Float%20%28single-precision%29) (DamageType :type Damage%20Type%20Object%20Reference) (InstigatedBy :type Controller%20Object%20Reference) (DamageCauser :type Actor%20Object%20Reference))
  (bind _asmy_player_state (Utilities|Casting|CastToMyPlayerState (Variables|/Script/Engine.Controller|GetPlayerState InstigatedBy))
    (:then
      (Default|IncrementScore _asmy_player_state)
      (Rendering|Material|SetVectorParameterValue (Variables|Default|Getdynamic%20material) "Color" (Utilities|Struct|MakeLinearColor 1.0 0.0 0.0 1.0) :!class /Script/Engine.MaterialInstanceDynamic)
      (Utilities|FlowControl|Delay 0.2)
      (Rendering|Material|SetVectorParameterValue (Variables|Default|Getdynamic%20material) "Color" (Utilities|Struct|MakeLinearColor 1.0 1.0 1.0 1.0) :!class /Script/Engine.MaterialInstanceDynamic))
    (:CastFailed
      (Development|PrintString "Hello"))))

(fn ConstructionScript)